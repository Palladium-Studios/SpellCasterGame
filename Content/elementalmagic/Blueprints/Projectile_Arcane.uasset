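; Arcane magic projectile that pushes physics objects and plays an impact effect when it stops.
; On hit, it applies a velocity-scaled impulse to simulating components at its own location, then destroys itself; other hits skip both steps.
; When projectile movement stops, it spawns an arcane impact emitter aligned to the surface normal, destroys a component and deactivates the Arcane and ArcaneTrail effects.
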(event OnProjectileStop(Projectile)
  (params (ImpactResult :type Hit%20Result%20Structure%20%28by%20ref%29))
  (bind (_bblockinghit _binitialoverlap _time _location _impactpoint _normal _impactnormal) (Collision|BreakHitResult ImpactResult))
  (Effects|SpawnEmitteratLocation "/Game/ElementalMagic/Particles/P_Impact_Arcane.P_Impact_Arcane" _location (Math|Conversions|RotationFromXVector _impactnormal))
  (Components|DestroyComponent)
  (Components|Activation|Deactivate (Variables|Default|GetArcane))
  (Components|Activation|Deactivate (Variables|Default|GetArcane_Trail)))

(event Collision|EventHit
  (params (MyComp :type Primitive%20Component%20Object%20Reference) (Other :type Actor%20Object%20Reference) (OtherComp :type Primitive%20Component%20Object%20Reference) (bSelfMoved :type Boolean) (HitLocation :type Vector :default "0, 0, 0") (HitNormal :type Vector :default "0, 0, 0") (NormalImpulse :type Vector :default "0, 0, 0") (Hit :type Hit%20Result%20Structure%20%28by%20ref%29))
  ;[1 1 1] d physics impulse to any physics object we hit
  (if (Physics|IsSimulatingPhysics OtherComp "None")
    (Physics|AddImpulseatLocation OtherComp (* (Transformation|GetVelocity) 1e+02) (Transformation|GetActorLocation) "None")
    (Actor|DestroyActor) ; Then destroy this projectile
  ))

(fn ConstructionScript)